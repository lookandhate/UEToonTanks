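; BP_TanksBaseGamemode is the tanks game mode Blueprint that shows the match start and end screens.
; The GameStart event creates a WBP_Gamestart widget, sets its start delay to three seconds and adds it to the viewport.
; The GameOver event creates a WBP_Gameend widget, passes it whether the local player won and adds it to the viewport.
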(event `self.GameStart`
  (`self.StartGameWidgetInit`))

(event `self.GameOver`
  (params (IsLocalPlayerWon :type Boolean))
  (`self.EndGameWidget` IsLocalPlayerWon))

(fn `EndGameWidget`
  (params (isPlayerWon :type Boolean))
  (bind _returnvalue (`|CreateWidget` "/Game/Blueprints/Widgets/WBP_Gameend.WBP_Gameend_C"))
  (`/Game/Blueprints/Widgets/WBP_Gameend.SetPlayerWon` _returnvalue isPlayerWon)
  (`UserWidget.AddToViewport` _returnvalue 0))

(fn `StartGameWidgetInit`
  (bind _returnvalue (`|CreateWidget` "/Game/Blueprints/Widgets/WBP_Gamestart.WBP_Gamestart_C"))
  (`/Game/Blueprints/Widgets/WBP_Gamestart.SetStartDelay` _returnvalue 3)
  (`UserWidget.AddToViewport` _returnvalue 0))

(fn `UserConstructionScript`)