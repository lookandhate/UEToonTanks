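; Speed power-up pickup that temporarily boosts the speed of a PawnTank that overlaps its box.
; On overlap it moves itself to a fixed world location, adds SpeedBoostAmount to the tank's current speed, then subtracts it after a hard-coded ten-second retriggerable delay and destroys itself.
; BoostTimeRemaining is initialized from MaxBoostTime at BeginPlay but does not drive the delay.
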(event `self.ReceiveBeginPlay`
  (`parent.ReceiveBeginPlay`)
  (set `self.BoostTimeRemaining` (`self.MaxBoostTime`)))

(event `self.Box.OnComponentBeginOverlap`
  (params (OverlappedComponent :type "PrimitiveComponent Object Reference") (OtherActor :type "Actor Object Reference") (OtherComp :type "PrimitiveComponent Object Reference") (OtherBodyIndex :type Integer) (bFromSweep :type Boolean) (SweepResult :type "HitResult Structure (by ref)"))
  (bind _as_pawn_tank (`self.As Pawn Tank`))
  (bind _aspawn_tank (cast `PawnTank` OtherActor))
  (bind _output_get (set `self.As Pawn Tank` _aspawn_tank))
  (`self.K2_SetActorLocation` (0.0 0.0 500.0))
  (`PawnTank.SetSpeed` _as_pawn_tank (+ (`PawnTank.GetCurrentSpeed` _output_get) (`self.SpeedBoostAmount`)))
  (`KismetSystemLibrary.RetriggerableDelay` 10.0)
  (`PawnTank.SetSpeed` _as_pawn_tank (- (`PawnTank.GetCurrentSpeed` _as_pawn_tank) (`self.SpeedBoostAmount`)))
  (`self.K2_DestroyActor`))

(fn `UserConstructionScript`
  (`parent.UserConstructionScript`))